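; Race start actor that runs a timed traffic-light countdown, then later turns into a finish marker.
; On BeginPlay, chained delays show red, yellow and green lights in turn, destroying the Box component on green.
; After a longer delay, green hides and the static mesh swaps to SM_Finish.
; Separately, a Master_Cart hitting Box1 makes its Gameplay_PC controller call AddMeOnList.
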(event OnComponentHit(Box1)
  (params (HitComponent :type Primitive%20Component%20Object%20Reference) (OtherActor :type Actor%20Object%20Reference) (OtherComp :type Primitive%20Component%20Object%20Reference) (NormalImpulse :type Vector :default "0, 0, 0") (Hit :type Hit%20Result%20Structure%20%28by%20ref%29))
  (bind _asmaster_cart (Utilities|Casting|CastToMaster_Cart OtherActor))
  (bind _asgameplay_pc (Utilities|Casting|CastToGameplay_PC (Pawn|GetController _asmaster_cart)))
  (Default|AddMeonList _asgameplay_pc))

(event EventBeginPlay
  (bind _yellowlight (Variables|Default|GetYellowlight))
  (bind _greenlight (Variables|Default|GetGreenLight))
  (bind _redlight (Variables|Default|GetRedLight))
  (Rendering|SetVisibility (Variables|Default|GetYellowlight) false false)
  (Utilities|FlowControl|Delay 2.0)
  (Rendering|SetVisibility _redlight true false)
  (Utilities|FlowControl|Delay 2.0)
  (Rendering|SetVisibility _redlight false false)
  (Rendering|SetVisibility _yellowlight true false)
  (Utilities|FlowControl|Delay 2.0)
  (Rendering|SetVisibility _yellowlight false false)
  (Rendering|SetVisibility _greenlight true false)
  (Components|DestroyComponent (Variables|Default|GetBox))
  (Utilities|FlowControl|Delay 15.0)
  (Rendering|SetVisibility _greenlight false false)
  (Components|StaticMesh|SetStaticMesh (Variables|Default|GetStaticMesh) "/Game/Models/TrackParts/Props/SM_Finish.SM_Finish"))

(fn ConstructionScript)