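; Spline actor that ranks MasterCart karts by race position along the track.
; It gathers all karts three seconds after BeginPlay, then each Tick reseeds their race length from spline length and distance to the first point, calling CalculateDistance per kart.
; CalculateDistance adjusts race length by distance to each kart's target point, advances nearby targets, then sorts ascending to assign positions and writes a last checkpoint location.
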(event Custom|ServerAddpos
  (bind _spline (Variables|Default|GetSpline))
  (for _array_element (Variables|Default|GetCars)
    (Utilities|IsValid _array_element
      (:Is%20Valid
        (Variables|/Game/Blueprints/Carts/ArcadeCarts/MasterCart.MasterCart_C|SetLastDistance _array_element (Math|Vector|VectorLength (- (Spline|GetLocationatSplinePoint _spline 0 "World") (Transformation|GetActorLocation _array_element))))
        (Variables|/Game/Blueprints/Carts/ArcadeCarts/MasterCart.MasterCart_C|SetRaceLenght _array_element (+ (Spline|GetSplineLength _spline) (Math|Vector|VectorLength (- (Spline|GetLocationatSplinePoint _spline 0 "World") (Transformation|GetActorLocation _array_element)))))
        (CallFunction|CalculateDistance)))))

(event EventBeginPlay
  (Utilities|FlowControl|Delay 3.0)
  (bind _outactors (Actor|GetAllActorsOfClass "/Game/Blueprints/Carts/ArcadeCarts/MasterCart.MasterCart_C"))
  (for _array_element _outactors
    (Utilities|Array|Add (Variables|Default|GetCars) _array_element)))

(event EventTick
  (params (DeltaSeconds :type Float%20%28single-precision%29))
  (CallFunction|ServerAddpos))

(fn ConstructionScript)

(fn CalculateDistance
  (bind _cars (Variables|Default|GetCars))
  (for (_array_element _array_index) _cars
    (Utilities|IsValid _array_element
      (:Is%20Valid
        (Variables|/Game/Blueprints/Carts/ArcadeCarts/MasterCart.MasterCart_C|Setposition _array_element _array_index)
        (Variables|/Game/Blueprints/Carts/ArcadeCarts/MasterCart.MasterCart_C|SetRaceLenght _array_element (- (Variables|/Game/Blueprints/Carts/ArcadeCarts/MasterCart.MasterCart_C|GetRaceLenght _array_element) (- (Variables|/Game/Blueprints/Carts/ArcadeCarts/MasterCart.MasterCart_C|GetLastDistance _array_element) (Math|Vector|VectorLength (- (Spline|GetLocationatSplinePoint (Variables|Default|GetSpline) (Variables|/Game/Blueprints/Carts/ArcadeCarts/MasterCart.MasterCart_C|GetDistantPoint _array_element) "World") (Transformation|GetActorLocation _array_element))))))
        (bind _output_get (Variables|/Game/Blueprints/Carts/ArcadeCarts/MasterCart.MasterCart_C|SetLastDistance _array_element (Math|Vector|VectorLength (- (Spline|GetLocationatSplinePoint (Variables|Default|GetSpline) (Variables|/Game/Blueprints/Carts/ArcadeCarts/MasterCart.MasterCart_C|GetDistantPoint _array_element) "World") (Transformation|GetActorLocation _array_element)))))
        (if (< _output_get 5e+02)
          (Variables|/Game/Blueprints/Carts/ArcadeCarts/MasterCart.MasterCart_C|SetDistantPoint _array_element (+ (Variables|/Game/Blueprints/Carts/ArcadeCarts/MasterCart.MasterCart_C|GetDistantPoint _array_element) 1))
          (Variables|/Game/Blueprints/Carts/ArcadeCarts/MasterCart.MasterCart_C|SetLastDistance _array_element (Math|Vector|VectorLength (- (Spline|GetLocationatSplinePoint (Variables|Default|GetSpline) (Variables|/Game/Blueprints/Carts/ArcadeCarts/MasterCart.MasterCart_C|GetDistantPoint _array_element) "World") (Transformation|GetActorLocation _array_element))))))))
  (for (_array_element_2 _array_index_2) (Class|LowEntryExtendedStandardLibrary|SortObjectArray _cars (EventDispatchers|CreateEvent :!event Sort) false)
    (bind _asmaster_cart (Utilities|Casting|CastToMasterCart _array_element_2))
    (Variables|/Game/Blueprints/Carts/ArcadeCarts/MasterCart.MasterCart_C|Setposition _asmaster_cart (+ _array_index_2 1))
    (Variables|/Game/Blueprints/Carts/ArcadeCarts/MasterCart.MasterCart_C|SetLastCheckpointlocation _asmaster_cart (Transformation|GetActorLocation _array_element))))

(fn Sort
  (params (ObjectA :type Object%20Object%20Reference) (ObjectB :type Object%20Object%20Reference))
  (bind _asmaster_cart (Utilities|Casting|CastToMasterCart ObjectA))
  (bind _asmaster_cart_2 (Utilities|Casting|CastToMasterCart ObjectB))
  (return (< (Variables|/Game/Blueprints/Carts/ArcadeCarts/MasterCart.MasterCart_C|GetRaceLenght _asmaster_cart) (Variables|/Game/Blueprints/Carts/ArcadeCarts/MasterCart.MasterCart_C|GetRaceLenght _asmaster_cart_2))))