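; FenceSpline is a Blueprint actor that builds segments for a fence along a spline in its construction script, with no active runtime logic.
; Section length comes from the RoadSplineMesh local X bounds plus SectionRarity, and spline length divided by it gives the segment count.
; A loop computes each segment's start and end distances and adds a SplineMeshComponent, but the visible graph never assigns its mesh or endpoints.
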(event EventBeginPlay)

(event Collision|EventActorBeginOverlap
  (params (OtherActor :type Actor%20Object%20Reference)))

(event EventTick
  (params (DeltaSeconds :type Float%20%28single-precision%29)))

(fn ConstructionScript
  (bind _roadsplinemesh (Variables|Default|GetRoadSplineMesh))
  (bind (_min _max) (Components|StaticMesh|GetLocalBounds _roadsplinemesh))
  (Utilities|FlowControl|Sequence
    (:then_0
      (bind _output_get (Variables|Default|SetMesh%20Bound%20size (- _max _min)))
      (Variables|Default|SetSection%20Lenght (+ (.x _output_get) (Variables|Default|GetSectionRarity))))
    (:then_1
      (bind _output_get_2 (Variables|Default|SetNumber%20of%20parts (.ReturnValue (Math|Float|Division(WholeandRemainder) (Spline|GetSplineLength (Variables|Default|GetSpline)) (Variables|Default|GetSection%20Lenght)))))
      (for _index (range 0 _output_get_2)
        (Variables|Default|SetDistanceStart (* _index (Variables|Default|GetSection%20Lenght)))
        (Variables|Default|SetDistance%20End (+ (* _index (Variables|Default|GetSection%20Lenght)) (Variables|Default|GetSection%20Lenght)))
        (bind _returnvalue (AddComponent|AddSplineMeshComponent true))
        (Variables|Default|SetNew%20Mesh _returnvalue)))))