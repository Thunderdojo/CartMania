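; Race start gate actor that runs a traffic-light countdown and later becomes the finish line.
; BeginPlay uses timed delays to call Wait on Gameplay_GM, cycle red, yellow and green lights, drop the Box barrier's collision and trigger the game mode's Start.
; After a further delay it swaps to the finish mesh and enables Box1, whose overlap calls AddMeOnList on the Master_Cart's Gameplay_PC controller.
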(event OnComponentBeginOverlap(Box1)
  (params (OverlappedComponent :type Primitive%20Component%20Object%20Reference) (OtherActor :type Actor%20Object%20Reference) (OtherComp :type Primitive%20Component%20Object%20Reference) (OtherBodyIndex :type Integer) (bFromSweep :type Boolean) (SweepResult :type Hit%20Result%20Structure%20%28by%20ref%29))
  (bind _asmaster_cart (Utilities|Casting|CastToMaster_Cart OtherActor))
  (bind _asgameplay_pc (Utilities|Casting|CastToGameplay_PC (Pawn|GetController _asmaster_cart)))
  (Default|AddMeonList _asgameplay_pc))

(event Custom|Startup!
  (bind _asgameplay_gm (Utilities|Casting|CastToGameplay_GM (Game|GetGameMode)))
  (Default|Start! _asgameplay_gm))

(event Custom|call%20wait
  (bind _asgameplay_gm (Utilities|Casting|CastToGameplay_GM (Game|GetGameMode)))
  (Default|Wait _asgameplay_gm))

(event EventBeginPlay
  (bind _yellowlight (Variables|Default|GetYellowlight))
  (bind _greenlight (Variables|Default|GetGreenLight))
  (bind _redlight (Variables|Default|GetRedLight))
  (bind _box1 (Variables|Default|GetBox1))
  (bind _box1_2 (Variables|Default|GetBox1))
  (Collision|SetCollisionEnabled _box1_2 "NoCollision")
  (Components|Activation|Deactivate _box1_2)
  (Utilities|FlowControl|Delay 1.0)
  (CallFunction|CallWait)
  (Rendering|SetVisibility (Variables|Default|GetYellowlight) false false)
  (Utilities|FlowControl|Delay 2.0)
  (Rendering|SetVisibility _redlight true false)
  (Utilities|FlowControl|Delay 2.0)
  (Rendering|SetVisibility _redlight false false)
  (Rendering|SetVisibility _yellowlight true false)
  (Utilities|FlowControl|Delay 2.0)
  (Rendering|SetVisibility _yellowlight false false)
  (Rendering|SetVisibility _greenlight true false)
  (Collision|SetCollisionEnabled (Variables|Default|GetBox) "NoCollision")
  (CallFunction|Startup!)
  (Utilities|FlowControl|Delay 15.0)
  (Rendering|SetVisibility _greenlight false false)
  (Components|StaticMesh|SetStaticMesh (Variables|Default|GetStaticMesh) "/Game/Models/TrackParts/Props/SM_Finish.SM_Finish")
  (Components|Activation|Activate _box1 true)
  (Collision|SetCollisionEnabled _box1 "QueryAndPhysics"))

(fn ConstructionScript)