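; Cart animator Blueprint that procedurally animates an arcade cart's static meshes, deferring entirely to its parent C++ ApplyAnimation for speed.
; An unconnected reference graph mirrors the native logic and can replace the parent call.
; It applies roll and tilt to the visuals mesh, then loops the wheel registry, setting each wheel's side-corrected spin, swing and vertical offset, plus steering yaw on steering wheels.
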(fn ApplyAnimation
  ;[0.6172 1 0] Most possible basic animation for the static mesh animator. The same thing is implemented in C++, so you can take a look there too.
  ;;[0 0.01562 1] The reason why below graph is not used is because the same logic is also implemented in C++, which is much faster for calculations like this. But if you want to create animation graph like this, feel free to remove Parent: Apply Animation node, and connect the graph you see below, and animation will just work the same way!
  (|CallParentFunction))