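; Game mode for the results screen, which shows race standings and characters matching each player's team.
; It collects controllers as they are swapped in and accumulates player info through AddInfo.
; Each update pushes the list to every ResultPC's HUD race list, removing the first entry once per controller beforehand.
; It then uses finishing position to index the ResultChar actors found, setting their team selection and calling ServerChange.
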(event Custom|AddInfo
  (params (PlayerInfo :type Player%20Info%20Structure))
  (CallFunction|Updateall PlayerInfo))

(event Custom|Updateall
  (params (Player%20info :type Player%20Info%20Structure%20%28by%20ref%29))
  (bind _allplayerinfo (Variables|Default|GetAllPlayerInfo))
  (Utilities|Array|Add (Variables|Default|GetAllPlayerInfo) Player%20info)
  (for _array_element (Variables|Default|GetAllPlayercontroller)
    (bind _asresult_pc (Utilities|Casting|CastToResultPC _array_element))
    (Utilities|Array|RemoveIndex _allplayerinfo)
    (Default|Update (Variables|/Game/UI/Results/ResultHud.ResultHud_C|GetRaceList (Variables|/Game/Blueprints/Results/ResultPC.ResultPC_C|GethudRef _asresult_pc)) _allplayerinfo))
  (bind _outactors (Actor|GetAllActorsOfClass "/Game/Blueprints/Results/ResultChar.ResultChar_C"))
  (for _array_element_2 (Variables|Default|GetAllPlayerInfo)
    (Utilities|IsValid (Utilities|Array|Get(acopy) _outactors (- (.LastPosition (Utilities|Struct|BreakPlayerInfo _array_element_2)) 1))
      (:Is%20Valid
        (Variables|/Game/Blueprints/Results/ResultChar.ResultChar_C|SetSelection (Utilities|Array|Get(acopy) _outactors (- (.LastPosition (Utilities|Struct|BreakPlayerInfo _array_element_2)) 1)) (.PlayerTeam (Utilities|Struct|BreakPlayerInfo _array_element_2)))
        (Default|ServerChange (Utilities|Array|Get(acopy) _outactors (- (.LastPosition (Utilities|Struct|BreakPlayerInfo _array_element_2)) 1)))))))

(event EventOnSwapPlayerControllers
  (params (OldPC :type Player%20Controller%20Object%20Reference) (NewPC :type Player%20Controller%20Object%20Reference))
  (Utilities|Array|Add (Variables|Default|GetAllPlayercontroller) NewPC))

(fn ConstructionScript)