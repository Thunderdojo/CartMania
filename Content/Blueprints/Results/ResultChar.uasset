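; Results character actor that displays a team's animal mascot with its idle animation, based on the Selection enum.
; The construction script sets the mesh and animation, and Changeall repeats that switch at runtime when called directly or through ServerChange.
; None and Team Rooster clear both mesh and animation.
; Changeall uses a looping PlayAnimation for Donkey, unlike the OverrideAnimationData used elsewhere.
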(event Custom|Changeall
  (bind _mesh (Variables|Character|GetMesh))
  (bind _mesh_2 (Variables|Character|GetMesh))
  (bind _mesh_3 (Variables|Character|GetMesh))
  (bind _mesh_4 (Variables|Character|GetMesh))
  (bind _mesh_5 (Variables|Character|GetMesh))
  (bind _mesh_6 (Variables|Character|GetMesh))
  (bind _mesh_7 (Variables|Character|GetMesh))
  (bind _mesh_8 (Variables|Character|GetMesh))
  (bind _mesh_9 (Variables|Character|GetMesh))
  (switch Utilities|FlowControl|Switch|SwitchonTeamEnum (Variables|Default|GetSelection)
    (:NewEnumerator0
      (Class|SkinnedMeshComponent|SetSkeletalMesh _mesh_5 0 true)
      (Components|Animation|OverrideAnimationData _mesh_5 0 true true 0.0 1.0))
    (:NewEnumerator1
      (Class|SkinnedMeshComponent|SetSkeletalMesh _mesh_9 "/Game/Models/Characters/Turtle/Turtle.Turtle" true)
      (Components|Animation|OverrideAnimationData _mesh_9 "/Game/Models/Characters/Turtle/TurtleIdle.TurtleIdle" true true 0.0 1.0))
    (:NewEnumerator2
      (Class|SkinnedMeshComponent|SetSkeletalMesh _mesh_6 "/Game/Models/Characters/Racoon/Racoon.Racoon" true)
      (Components|Animation|OverrideAnimationData _mesh_6 "/Game/Models/Characters/Racoon/Racoon_Idle.Racoon_Idle" true true 0.0 1.0))
    (:NewEnumerator3
      (Class|SkinnedMeshComponent|SetSkeletalMesh _mesh_7 "/Game/Models/Characters/Gator/Gator.Gator" true)
      (Components|Animation|OverrideAnimationData _mesh_7 "/Game/Models/Characters/Gator/Ali_lobby_idle.Ali_lobby_idle" true true 0.0 1.0))
    (:NewEnumerator4
      (Class|SkinnedMeshComponent|SetSkeletalMesh _mesh_8 "/Game/Models/Characters/Duck/Ducky.Ducky" true)
      (Components|Animation|OverrideAnimationData _mesh_8 "/Game/Models/Characters/Duck/Duckidle.Duckidle" true true 0.0 1.0))
    (:NewEnumerator5
      (Class|SkinnedMeshComponent|SetSkeletalMesh _mesh_3 "/Game/Models/Characters/Monkey/Monkey.Monkey" true)
      (Components|Animation|OverrideAnimationData _mesh_3 "/Game/Models/Characters/Monkey/MonkeyIdle_Anim.MonkeyIdle_Anim" true true 0.0 1.0))
    (:NewEnumerator6
      (Class|SkinnedMeshComponent|SetSkeletalMesh _mesh_4 "/Game/Models/Characters/Beaver/beaver.beaver" true)
      (Components|Animation|OverrideAnimationData _mesh_4 "/Game/Models/Characters/Beaver/BeaverIdle_Anim.BeaverIdle_Anim" true true 0.0 1.0))
    (:NewEnumerator7
      (Class|SkinnedMeshComponent|SetSkeletalMesh _mesh_2 0 true)
      (Components|Animation|OverrideAnimationData _mesh_2 0 true true 0.0 1.0))
    (:NewEnumerator8
      (Class|SkinnedMeshComponent|SetSkeletalMesh _mesh "/Game/Models/Characters/Donkey/Donkey.Donkey" true)
      (Components|Animation|PlayAnimation _mesh "/Game/Models/Characters/Donkey/DonkeyIdle.DonkeyIdle" true))))

(event Custom|ServerChange
  (CallFunction|Changeall))

(event EventBeginPlay)

(event Collision|EventActorBeginOverlap
  (params (OtherActor :type Actor%20Object%20Reference)))

(event EventTick
  (params (DeltaSeconds :type Float%20%28single-precision%29)))

(fn ConstructionScript
  (bind _mesh (Variables|Character|GetMesh))
  (bind _mesh_2 (Variables|Character|GetMesh))
  (bind _mesh_3 (Variables|Character|GetMesh))
  (bind _mesh_4 (Variables|Character|GetMesh))
  (bind _mesh_5 (Variables|Character|GetMesh))
  (bind _mesh_6 (Variables|Character|GetMesh))
  (bind _mesh_7 (Variables|Character|GetMesh))
  (bind _mesh_8 (Variables|Character|GetMesh))
  (bind _mesh_9 (Variables|Character|GetMesh))
  (switch Utilities|FlowControl|Switch|SwitchonTeamEnum (Variables|Default|GetSelection)
    (:NewEnumerator0
      (Class|SkinnedMeshComponent|SetSkeletalMesh _mesh_5 0 true)
      (Components|Animation|OverrideAnimationData _mesh_5 0 true true 0.0 1.0))
    (:NewEnumerator1
      (Class|SkinnedMeshComponent|SetSkeletalMesh _mesh_9 "/Game/Models/Characters/Turtle/Turtle.Turtle" true)
      (Components|Animation|OverrideAnimationData _mesh_9 "/Game/Models/Characters/Turtle/TurtleIdle.TurtleIdle" true true 0.0 1.0))
    (:NewEnumerator2
      (Class|SkinnedMeshComponent|SetSkeletalMesh _mesh_6 "/Game/Models/Characters/Racoon/Racoon.Racoon" true)
      (Components|Animation|OverrideAnimationData _mesh_6 "/Game/Models/Characters/Racoon/Racoon_Idle.Racoon_Idle" true true 0.0 1.0))
    (:NewEnumerator3
      (Class|SkinnedMeshComponent|SetSkeletalMesh _mesh_7 "/Game/Models/Characters/Gator/Gator.Gator" true)
      (Components|Animation|OverrideAnimationData _mesh_7 "/Game/Models/Characters/Gator/Ali_lobby_idle.Ali_lobby_idle" true true 0.0 1.0))
    (:NewEnumerator4
      (Class|SkinnedMeshComponent|SetSkeletalMesh _mesh_8 "/Game/Models/Characters/Duck/Ducky.Ducky" true)
      (Components|Animation|OverrideAnimationData _mesh_8 "/Game/Models/Characters/Duck/Duckidle.Duckidle" true true 0.0 1.0))
    (:NewEnumerator5
      (Class|SkinnedMeshComponent|SetSkeletalMesh _mesh_3 "/Game/Models/Characters/Monkey/Monkey.Monkey" true)
      (Components|Animation|OverrideAnimationData _mesh_3 "/Game/Models/Characters/Monkey/MonkeyIdle_Anim.MonkeyIdle_Anim" true true 0.0 1.0))
    (:NewEnumerator6
      (Class|SkinnedMeshComponent|SetSkeletalMesh _mesh_4 "/Game/Models/Characters/Beaver/beaver.beaver" true)
      (Components|Animation|OverrideAnimationData _mesh_4 "/Game/Models/Characters/Beaver/BeaverIdle_Anim.BeaverIdle_Anim" true true 0.0 1.0))
    (:NewEnumerator7
      (Class|SkinnedMeshComponent|SetSkeletalMesh _mesh_2 0 true)
      (Components|Animation|OverrideAnimationData _mesh_2 0 true true 0.0 1.0))
    (:NewEnumerator8
      (Class|SkinnedMeshComponent|SetSkeletalMesh _mesh "/Game/Models/Characters/Donkey/Donkey.Donkey" true)
      (Components|Animation|OverrideAnimationData _mesh "/Game/Models/Characters/Donkey/DonkeyIdle.DonkeyIdle" true true 0.0 1.0))))