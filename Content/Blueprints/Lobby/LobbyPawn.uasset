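; Lobby pawn that displays a cart and an animal character for the selected team.
; ChangeCharacterandCart acts only when the given player controller matches the pawn's own Lobby_PC, then switches on the Team enum.
; Each team sets the cart's static mesh and the character's skeletal mesh with a looping idle, while None clears both meshes.
; The Rooster team uses Wabbit meshes and has no animation asset assigned.
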(event Custom|Change%20Character%20and%20Cart
  (params (Team :type TeamEnum%20Enum :default "NewEnumerator0") (Playercontroller :type Player%20Controller%20Object%20Reference))
  (bind _lobbycharacter (Variables|Default|GetLobbyCharacter))
  (bind _lobbycharacter_2 (Variables|Default|GetLobbyCharacter))
  (bind _lobbycharacter_3 (Variables|Default|GetLobbyCharacter))
  (bind _lobbycharacter_4 (Variables|Default|GetLobbyCharacter))
  (bind _lobbycharacter_5 (Variables|Default|GetLobbyCharacter))
  (bind _lobbycharacter_6 (Variables|Default|GetLobbyCharacter))
  (bind _lobbycharacter_7 (Variables|Default|GetLobbyCharacter))
  (bind _lobbycharacter_8 (Variables|Default|GetLobbyCharacter))
  ;[0.1965 1 0.008488] Sets Cart and Character on the values of the TEam Ennum
  (if (== (.AsLobby%20PC (Utilities|Casting|CastToLobby_PC (Pawn|GetController))) Playercontroller)
    (switch Utilities|FlowControl|Switch|SwitchonTeamEnum Team
      (:NewEnumerator0
        (Components|StaticMesh|SetStaticMesh (Variables|Default|GetLobbyCart) 0)
        (Class|SkinnedMeshComponent|SetSkeletalMesh (Variables|Default|GetLobbyCharacter) 0 true))
      (:NewEnumerator1
        (Components|StaticMesh|SetStaticMesh (Variables|Default|GetLobbyCart) "/Game/Models/Lobby/FullCarts/FullTurtleCart.FullTurtleCart")
        (Class|SkinnedMeshComponent|SetSkeletalMesh _lobbycharacter_6 "/Game/Models/Characters/Turtle/Turtle.Turtle" true)
        (Components|Animation|PlayAnimation _lobbycharacter_6 "/Game/Models/Characters/Turtle/TurtleIdle.TurtleIdle" true))
      (:NewEnumerator2
        (Components|StaticMesh|SetStaticMesh (Variables|Default|GetLobbyCart) "/Game/Models/Lobby/FullCarts/FullRacoonCart.FullRacoonCart")
        (Class|SkinnedMeshComponent|SetSkeletalMesh _lobbycharacter_7 "/Game/Models/Characters/Racoon/Racoon.Racoon" true)
        (Components|Animation|PlayAnimation _lobbycharacter_7 "/Game/Models/Characters/Racoon/Racoon_Idle.Racoon_Idle" true))
      (:NewEnumerator3
        (Components|StaticMesh|SetStaticMesh (Variables|Default|GetLobbyCart) "/Game/Models/Lobby/FullCarts/FullAliCart.FullAliCart")
        (Class|SkinnedMeshComponent|SetSkeletalMesh _lobbycharacter_8 "/Game/Models/Characters/Gator/Gator.Gator" true)
        (Components|Animation|PlayAnimation _lobbycharacter_8 "/Game/Models/Characters/Gator/Ali_lobby_idle.Ali_lobby_idle" true))
      (:NewEnumerator4
        (Components|StaticMesh|SetStaticMesh (Variables|Default|GetLobbyCart) "/Game/Models/Lobby/FullCarts/FullDuckCart.FullDuckCart")
        (Class|SkinnedMeshComponent|SetSkeletalMesh _lobbycharacter_2 "/Game/Models/Characters/Duck/Ducky.Ducky" true)
        (Components|Animation|PlayAnimation _lobbycharacter_2 "/Game/Models/Characters/Duck/Duckidle.Duckidle" true))
      (:NewEnumerator5
        (Components|StaticMesh|SetStaticMesh (Variables|Default|GetLobbyCart) "/Game/Models/Lobby/FullCarts/FullMonkeyCart.FullMonkeyCart")
        (Class|SkinnedMeshComponent|SetSkeletalMesh _lobbycharacter_3 "/Game/Models/Characters/Monkey/Monkey.Monkey" true)
        (Components|Animation|PlayAnimation _lobbycharacter_3 "/Game/Models/Characters/Monkey/MonkeyIdle_Anim.MonkeyIdle_Anim" true))
      (:NewEnumerator6
        (Components|StaticMesh|SetStaticMesh (Variables|Default|GetLobbyCart) "/Game/Models/Lobby/FullCarts/FullBeaverCart.FullBeaverCart")
        (Class|SkinnedMeshComponent|SetSkeletalMesh _lobbycharacter_4 "/Game/Models/Characters/Beaver/beaver.beaver" true)
        (Components|Animation|PlayAnimation _lobbycharacter_4 "/Game/Models/Characters/Beaver/BeaverIdle_Anim.BeaverIdle_Anim" true))
      (:NewEnumerator7
        (Components|StaticMesh|SetStaticMesh (Variables|Default|GetLobbyCart) "/Game/Models/Lobby/WabbitCartFull.WabbitCartFull")
        (Class|SkinnedMeshComponent|SetSkeletalMesh _lobbycharacter_5 "/Game/Models/Characters/Rabbit/wabbit.wabbit" true)
        (Components|Animation|PlayAnimation _lobbycharacter_5 0 true))
      (:NewEnumerator8
        (Components|StaticMesh|SetStaticMesh (Variables|Default|GetLobbyCart) "/Game/Models/Lobby/FullCarts/FullDonkeyCart.FullDonkeyCart")
        (Class|SkinnedMeshComponent|SetSkeletalMesh _lobbycharacter "/Game/Models/Characters/Donkey/Donkey.Donkey" true)
        (Components|Animation|PlayAnimation _lobbycharacter "/Game/Models/Characters/Donkey/DonkeyIdle.DonkeyIdle" true)))))

(fn ConstructionScript)